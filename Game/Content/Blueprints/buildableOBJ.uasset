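; A buildable object that changes its material once enough pickup actors have been placed over it, then consumes them.
; Overlap begin and end events keep a running count of overlapping pickups and print it.
; Tick checks whether the count exceeds ColNeeded, swaps the main mesh material, then after a short delay destroys the overlapping pickups in two successive passes.
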(event EventBeginPlay
  (Variables|Default|SetcollCount 0.0))

(event EventTick
  (params (DeltaSeconds :type Float%20%28single-precision%29))
  (bind _overlappingactors (Collision|GetOverlappingActors "/Game/Blueprints/pickup.pickup_C" :!class /Script/Engine.Actor))
  (if (> (Variables|Default|GetcollCount) (Variables|Default|GetcolNeeded))
    (Rendering|Material|SetMaterial (Variables|Default|GetmainMesh) 0 "/Game/Materials/whatever.whatever")
    (Utilities|FlowControl|Delay 0.1)
    (for _array_element _overlappingactors
      (Actor|DestroyActor _array_element))
    (for _array_element_2 _overlappingactors
      (Actor|DestroyActor _array_element_2))))

(event Collision|EventActorBeginOverlap
  (params (OtherActor :type Actor%20Object%20Reference))
  (Utilities|Casting|CastTopickup OtherActor)
  (bind _output_get (Variables|Default|SetcollCount (+ (Variables|Default|GetcollCount) 1)))
  (Development|PrintText (Utilities|Text|ToText(Float) _output_get "HalfToEven")))

(event Collision|EventActorEndOverlap
  (params (OtherActor :type Actor%20Object%20Reference))
  (Utilities|Casting|CastTopickup OtherActor)
  (bind _output_get (Variables|Default|SetcollCount (- (Variables|Default|GetcollCount) 1)))
  (Development|PrintText (Utilities|Text|ToText(Float) _output_get "HalfToEven")))

(fn ConstructionScript)