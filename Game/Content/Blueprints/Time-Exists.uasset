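; Actor for a time-shift mechanic that makes a spawned counterpart appear and disappear on player input.
; On BeginPlay it enables input and spawns an actor of the class taken from Object at its own transform.
; Each TimeShift press flips Exists, setting the spawned actor's visibility through child components and enabling or disabling its input.
; The toggle leaves collision untouched and never destroys the spawned actor.
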(event EventBeginPlay
  (Input|EnableInput (Game|GetPlayerController 0))
  (bind _returnvalue (Game|SpawnActorfromClass (Utilities|GetClass (Variables|Default|Getobject)) (Transformation|GetActorTransform) "Undefined" "MultiplyWithRoot" 0 0)))

(event Input|ActionEvents|InputActionTimeShift
  (params (Key :type Key%20Structure :default "None"))
  (bind _returnvalue (Game|GetPlayerController 0))
  (:Pressed
    (Utilities|FlowControl|FlipFlop
      (:A
        (bind _output_get (Variables|Default|Setexists true))
        (Rendering|SetVisibility (Variables|/Script/Engine.Actor|GetRootComponent (stale EventBeginPlay _returnvalue)) _output_get true)
        (Input|EnableInput (stale EventBeginPlay _returnvalue) _returnvalue))
      (:B
        (bind _output_get_2 (Variables|Default|Setexists false))
        (Rendering|SetVisibility (Variables|/Script/Engine.Actor|GetRootComponent (stale EventBeginPlay _returnvalue)) _output_get_2 true)
        (Input|DisableInput (stale EventBeginPlay _returnvalue) _returnvalue)))))

(fn ConstructionScript)