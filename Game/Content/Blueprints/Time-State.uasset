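; Time-State actor that lets the player toggle between two world states by pressing G.
; It enables input for the first player controller on BeginPlay, and a FlipFlop on G sets the State boolean.
; Each toggle spawns an actor of State1's or State2's class at this actor's transform, then destroys the one spawned for the other state.
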(event EventBeginPlay
  (Input|EnableInput (Game|GetPlayerController 0)))

(event Input|KeyboardEvents|G
  (params (Key :type Key%20Structure :default "None"))
  (:Pressed
    (Utilities|FlowControl|FlipFlop
      (:A
        (Variables|Default|Setstate true))
      (:B
        (Variables|Default|Setstate false)))
    (if (Variables|Default|Getstate)
      (bind _returnvalue (Game|SpawnActorfromClass (Utilities|GetClass (Variables|Default|Getstate1)) (Transformation|GetActorTransform) "Undefined" "MultiplyWithRoot" 0 0))
      (Actor|DestroyActor (stale _returnvalue_2))
      (else
        (bind _returnvalue_2 (Game|SpawnActorfromClass (Utilities|GetClass (Variables|Default|Getstate2)) (Transformation|GetActorTransform) "Undefined" "MultiplyWithRoot" 0 0))
        (Actor|DestroyActor _returnvalue)))))

(fn ConstructionScript)