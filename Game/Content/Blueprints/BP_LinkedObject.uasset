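; BP_LinkedObject makes a Linked actor follow a Parent actor at a fixed world-space offset, without attachment.
; BeginPlay caches the location offset between the two actors.
; Each Tick compares Parent location plus offset to the last applied position and, beyond a small tolerance, teleport-free and without sweep moves Linked there and copies Parent's rotation.
; The offset does not rotate, and rotation alone triggers no update.
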(event EventBeginPlay
  (bind _linked (Variables|Default|GetLinked))
  (bind _returnvalue (Transformation|GetActorLocation _linked))
  (Variables|Default|SetOffset (- _returnvalue (Transformation|GetActorLocation (Variables|Default|GetParent))))
  (Variables|Default|SetPrevPos _returnvalue))

(event EventTick
  (params (DeltaSeconds :type Float%20%28single-precision%29))
  (bind _parent (Variables|Default|GetParent))
  (bind _linked (Variables|Default|GetLinked))
  (bind _offset (Variables|Default|GetOffset))
  (bind _returnvalue (Transformation|GetActorLocation _parent))
  (bind _returnvalue_2 (+ _offset _returnvalue))
  (if (Utilities|Operators|NotEqual(!=) (Variables|Default|GetPrevPos) _returnvalue_2 5.0)
    (Transformation|SetActorLocation _linked _returnvalue_2 false false)
    (Variables|Default|SetPrevPos _returnvalue_2)
    (Transformation|SetActorRotation _linked (Transformation|GetActorRotation (Variables|Default|GetParent)))))